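; BP_Bobber is a fishing bobber that drops onto animated water and floats, its line cable attached to the player character's mesh at BeginPlay.
; Each Tick syncs a wave offset and, until in water, tests for surface contact.
; Contact writes impact location and time to the MPC_GlobalWater parameter collection, stops physics and stores XY.
; Afterwards it follows the wave height, dips via the Wippen timeline and smooths its rotation.
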(event EventTick
  (params (DeltaSeconds :type Float%20%28single-precision%29))
  (bind (_returnvalue_x _returnvalue_y _returnvalue_z _returnvalue) (|CheckSurfaceIntersection))
  (Variables|Default|SetWellenOffset (|Math_Wellenhöhesynchronisieren))
  (if (Variables|Default|GetImWasser)
    (|UpdateWaterPhysics)
    (else
      (|UpdateGlobalMaterialParameters (<= _returnvalue_z _returnvalue))
      (|EnterWaterState _returnvalue_x _returnvalue_y))))

(fn ConstructionScript)

(event EventBeginPlay
  (Class|CableComponent|SetAttachEndto (Variables|Default|GetCable) (Game|GetPlayerCharacter 0) "Mesh" "None"))