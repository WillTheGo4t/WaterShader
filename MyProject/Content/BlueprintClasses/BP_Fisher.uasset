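; BP_Fisher is the player-controlled fisher, able to walk, look around and cast a fishing bobber.
; Axis inputs drive movement along the actor's forward and right vectors, while mouse input turns the controller with inverted pitch input.
; Left click toggles the cast: it destroys an existing bobber, or spawns BP_Bobber above the camera and launches it along the view direction with a mass-independent velocity-change impulse.
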(fn ConstructionScript)

(event Input|AxisEvents|InputAxisMoveForward
  (params (AxisValue :type Float%20%28single-precision%29))
  (Pawn|Input|AddMovementInput (Transformation|GetActorForwardVector) AxisValue false))

(event Input|AxisEvents|InputAxisMoveSide
  (params (AxisValue :type Float%20%28single-precision%29))
  (Pawn|Input|AddMovementInput (Transformation|GetActorRightVector) AxisValue false))

(event Input|MouseEvents|MouseX
  (params (AxisValue :type Float%20%28single-precision%29))
  (Pawn|Input|AddControllerYawInput AxisValue))

(event Input|MouseEvents|MouseY
  (params (AxisValue :type Float%20%28single-precision%29))
  (Pawn|Input|AddControllerPitchInput (* AxisValue -1.0)))

(event Input|MouseEvents|LeftMouseButton
  (params (Key :type Key%20Structure :default "None"))
  (bind _camera (Variables|Default|GetCamera))
  (:Pressed
    (bind _mybobber (Variables|Default|GetMyBobber)
      (:then
        (Actor|DestroyActor _mybobber))
      (:else
        (bind _returnvalue (Game|SpawnActorfromClass "/Game/BlueprintClasses/BP_Bobber.BP_Bobber_C" (Math|Transform|MakeTransform (+ (Transformation|GetWorldLocation _camera) "0.000000,0.000000,60.000000") (Transformation|GetWorldRotation _camera) "1.000000,1.000000,1.000000") "AlwaysSpawn" "MultiplyWithRoot" 0 0))
        (bind _output_get (Variables|Default|SetMyBobber _returnvalue))
        (Physics|AddImpulse (Variables|/Game/BlueprintClasses/BP_Bobber.BP_Bobber_C|GetSphere _output_get) (* (Math|Vector|GetForwardVector _camera) "1500.000000,1500.000000,1500.000000") "None" true)))))